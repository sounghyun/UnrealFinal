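; Player hero character with axis-driven movement, punching and an equippable gun.
; BeginPlay shows the cursor and spawns a MousePointBP marker, which left clicks move to the location under the cursor.
; Hand-socketed spheres call DoorHit on doors they begin overlapping while punch input is held.
; GunSet spawns GunBP once onto GunSocket, zeroes its rotating movement and sets GunOn, which disables punch input.
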(event OnComponentBeginOverlap(Sphere)
  (params (OverlappedComponent :type Primitive%20Component%20Object%20Reference) (OtherActor :type Actor%20Object%20Reference) (OtherComp :type Primitive%20Component%20Object%20Reference) (OtherBodyIndex :type Integer) (bFromSweep :type Boolean) (SweepResult :type Hit%20Result%20Structure%20%28by%20ref%29))
  (bind _asdoor (Utilities|Casting|CastTodoor OtherActor))
  (if (Variables|Default|GetPunching)
    (Default|DoorHit _asdoor)))

(event OnComponentBeginOverlap(Sphere1)
  (params (OverlappedComponent :type Primitive%20Component%20Object%20Reference) (OtherActor :type Actor%20Object%20Reference) (OtherComp :type Primitive%20Component%20Object%20Reference) (OtherBodyIndex :type Integer) (bFromSweep :type Boolean) (SweepResult :type Hit%20Result%20Structure%20%28by%20ref%29))
  (bind _asdoor (Utilities|Casting|CastTodoor OtherActor))
  (if (Variables|Default|GetPunching)
    (Default|DoorHit _asdoor)))

(event Custom|GunSet
  (if (not (Variables|Default|GetGunOn))
    (bind _returnvalue (Game|SpawnActorfromClass "/Game/Gun/GunBP.GunBP_C" (Transformation|GetWorldTransform (Variables|Character|GetMesh)) "Undefined" 0 0))
    (bind _output_get (Variables|Default|SetGun _returnvalue))
    (Transformation|AttachComponentToComponent _output_get (Variables|Character|GetMesh) "GunSocket" "SnapToTarget" "SnapToTarget" "KeepWorld" true)
    (Variables|Default|SetGunOn true)
    (Variables|/Script/Engine.RotatingMovementComponent|SetRotationRate (Variables|/Game/Gun/GunBP.GunBP_C|GetRotatingMovement _output_get) "0, 0, 0")))

(event EventBeginPlay
  (bind _returnvalue (Game|SpawnActorfromClass "/Game/UI/MousePointBP.MousePointBP_C" (Math|Conversions|ToTransform(Vector) (Transformation|GetActorLocation)) "Undefined" 0 0))
  (Variables|Default|SetMouseClickPoint _returnvalue)
  (Variables|/Script/Engine.PlayerController|SetbShowMouseCursor (Game|GetPlayerController 0) true))

(event Collision|EventActorBeginOverlap
  (params (OtherActor :type Actor%20Object%20Reference)))

(event EventTick
  (params (DeltaSeconds :type Float%20%28single-precision%29)))

(event Input|ActionEvents|InputActionLeftMouseClicked
  (params (Key :type Key%20Structure :default "AnyKey"))
  (:Pressed
    (Transformation|SetActorLocation (Variables|Default|GetMouseClickPoint) (.Location (Collision|BreakHitResult (.HitResult (Game|Player|GetHitResultUnderCursorbyChannel (Game|GetPlayerController 0) "TraceTypeQuery1" true)))) false false)))

(event Input|ActionEvents|InputActionPunchingAndFire
  (params (Key :type Key%20Structure :default "AnyKey"))
  (bind _gunon (Variables|Default|GetGunOn))
  (:Pressed
    (if (not _gunon)
      (Variables|Default|SetPunching true)))
  (:Released
    (if (not _gunon)
      (Variables|Default|SetPunching false))))

(event Input|AxisEvents|InputAxisUD
  (params (AxisValue :type Float%20%28single-precision%29))
  (Pawn|Input|AddMovementInput (Math|Vector|GetForwardVector (Pawn|GetControlRotation :!class /Script/Engine.Pawn)) AxisValue false))

(event Input|AxisEvents|InputAxisTurn
  (params (AxisValue :type Float%20%28single-precision%29)))

(event Input|AxisEvents|InputAxisLookup
  (params (AxisValue :type Float%20%28single-precision%29)))

(event Input|AxisEvents|InputAxisLR
  (params (AxisValue :type Float%20%28single-precision%29))
  (Pawn|Input|AddMovementInput (Math|Vector|GetRightVector (Pawn|GetControlRotation :!class /Script/Engine.Pawn)) AxisValue false))

(fn ConstructionScript
  (bind _mesh (Variables|Character|GetMesh))
  (Transformation|AttachComponentToComponent (Variables|Default|GetSphere1) _mesh "hand_l" "SnapToTarget" "SnapToTarget" "KeepWorld" true)
  (Transformation|AttachComponentToComponent (Variables|Default|GetSphere) _mesh "hand_r" "SnapToTarget" "SnapToTarget" "KeepWorld" true))