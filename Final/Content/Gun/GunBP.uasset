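; Gun actor that spawns Bullet actors at its Arrow component's transform, with automatic fire between FireStart and FireEnd.
; FireStart fires immediately and starts a looping timer on Fire, which FireEnd clears.
; The Box overlap only casts to HeroBP; nodes to stop RotatingMovement and call GunSet are left unconnected, so that overlap has no effect yet.
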(event OnComponentBeginOverlap(Box)
  (params (OverlappedComponent :type Primitive%20Component%20Object%20Reference) (OtherActor :type Actor%20Object%20Reference) (OtherComp :type Primitive%20Component%20Object%20Reference) (OtherBodyIndex :type Integer) (bFromSweep :type Boolean) (SweepResult :type Hit%20Result%20Structure%20%28by%20ref%29))
  (Utilities|Casting|CastToHeroBP OtherActor))

(event Custom|Fire
  (Game|SpawnActorfromClass "/Game/Gun/bullet.bullet_C" (Transformation|GetWorldTransform (Variables|Default|GetArrow)) "Undefined" 0 0))

(event Custom|FireStart
  (CallFunction|Fire)
  (Utilities|Time|SetTimerbyFunctionName 0 "Fire" 0.1 true))

(event Custom|FireEnd
  (Utilities|Time|ClearTimerbyFunctionName 0 "Fire"))

(event EventBeginPlay)

(event Collision|EventActorBeginOverlap
  (params (OtherActor :type Actor%20Object%20Reference)))

(event EventTick
  (params (DeltaSeconds :type Float%20%28single-precision%29)))

(fn ConstructionScript)